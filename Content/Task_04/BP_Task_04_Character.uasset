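; Test character demonstrating replication of a UObject and of a component created at runtime.
; On BeginPlay the server constructs a randomized BP_ObjectForReplication every five seconds and adds a replicated skeletal mesh component.
; CreatedComponent's OnRep assigns the TutorialTPP mesh once the component is valid.
; Tick prints the object's values and the component's name each frame to show the replicated state.
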(event `self.ReceiveBeginPlay`
  (if (`KismetSystemLibrary.IsServer`)
    (`|ExecutionSequence`
      (:`then_0`
        (bind _returnvalue (`|GenericCreateObject` "/Game/Task_04/BP_ObjectForReplication.BP_ObjectForReplication_C" (`KismetMathLibrary.RandomBool`) (`KismetMathLibrary.RandomFloat`) (`KismetMathLibrary.RandomInteger` 100) :!label _label))
        (set `self.ReplicatedObject` _returnvalue)
        (`KismetSystemLibrary.Delay` 5.0)
        (goto _label))
      (:`then_1`
        (bind _returnvalue_2 (`AddComponent|NODE_AddSkeletalMeshComponent-0`))
        (`ActorComponent.SetIsReplicated` _returnvalue_2 true)
        (set `self.CreatedComponent` _returnvalue_2)))))

(event `self.ReceiveTick`
  (params (DeltaSeconds :type "Float (single-precision)"))
  (`|ExecutionSequence`
    (:`then_0`
      (bind _replicatedobject (`self.ReplicatedObject`)
        (:`then`
          (bind _asbp_object_for_replication (cast `/Game/Task_04/BP_ObjectForReplication` _replicatedobject))
          (`KismetSystemLibrary.PrintString` (`KismetStringLibrary.Concat_StrStr` (`KismetStringLibrary.Conv_BoolToString` (`/Game/Task_04/BP_ObjectForReplication.Value1` _asbp_object_for_replication)) "  " (`KismetStringLibrary.Conv_DoubleToString` (`/Game/Task_04/BP_ObjectForReplication.Value2` _asbp_object_for_replication)) "  " (`KismetStringLibrary.Conv_IntToString` (`/Game/Task_04/BP_ObjectForReplication.Value3` _asbp_object_for_replication))) true true (struct :`G` 0.66 :`B` 1.0 :`A` 1.0) 0.0))
        (:`else`)))
    (:`then_1`
      (`KismetSystemLibrary.PrintString` (`KismetSystemLibrary.GetDisplayName` (`self.CreatedComponent`)) true true (struct :`R` 1.0 :`G` 0.389367 :`A` 1.0) 0.0))))

(fn `OnRep_CreatedComponent`
  (bind _createdcomponent (`self.CreatedComponent`)
    (:`then`
      (`SkeletalMeshComponent.SetSkeletalMeshAsset` _createdcomponent "/Engine/Tutorial/SubEditors/TutorialAssets/Character/TutorialTPP.TutorialTPP"))
    (:`else`)))

(fn `UserConstructionScript`)