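; Extendable robotic arm that grabs physics objects while the right mouse button is held and drops them on release.
; A physics handle pulls a sphere hand toward a forward target distance that extends while held and retracts otherwise.
; Simulating components the sphere hits are welded to it, then detached with their velocity preserved.
; Each tick bends spline points toward the sphere using squared lateral interpolation and stretches lazily created cylinder spline meshes along them.
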(event `self.ReceiveBeginPlay`
  (`PhysicsHandleComponent.GrabComponentAtLocation` (`self.PhysicsHandle`) (`self.Sphere`) "None" (`SceneComponent.K2_GetComponentLocation` (`self.Sphere`))))

(event `self.ReceiveTick`
  (params (DeltaSeconds :type "Float (single-precision)"))
  (bind _rmbpressed (`self.RMBPressed`))
  (bind _output_get (set `self.TargetDistance` (`KismetMathLibrary.FInterpTo_Constant` (`self.TargetDistance`) (`KismetMathLibrary.SelectFloat` 500.0 30.0 _rmbpressed) DeltaSeconds (`KismetMathLibrary.SelectFloat` 400.0 1000.0 _rmbpressed))))
  (`PhysicsHandleComponent.SetTargetLocation` (`self.PhysicsHandle`) (`KismetMathLibrary.TransformLocation` (`self.GetTransform`) (`KismetMathLibrary.MakeVector` _output_get)))
  (`self.UpdateSplinePoints`)
  (`self.UpdateSplineMesh`))

(event `RMB_Pressed`
  (set `self.RMBPressed` true))

(event `RMB_Released`
  (set `self.RMBPressed` false)
  (for _array_element (`self.AttachedComponents`)
    (`/Engine/EditorBlueprintResources/StandardMacros.IsValid` _array_element
      (:`Is Valid`
        (bind _returnvalue (`PrimitiveComponent.GetPhysicsLinearVelocity` _array_element "None"))
        (`SceneComponent.K2_DetachFromComponent` _array_element "KeepWorld" "KeepWorld" "KeepWorld" false)
        (`PrimitiveComponent.SetPhysicsLinearVelocity` _array_element _returnvalue false "None"))))
  (`KismetArrayLibrary.Array_Clear` (`self.AttachedComponents`)))

(event `self.Sphere.OnComponentHit`
  (params (HitComponent :type "PrimitiveComponent Object Reference") (OtherActor :type "Actor Object Reference") (OtherComp :type "PrimitiveComponent Object Reference") (NormalImpulse :type "Vector Structure") (Hit :type "HitResult Structure (by ref)"))
  (if (and (`self.RMBPressed`) (`SceneComponent.IsSimulatingPhysics` OtherComp "None"))
    (`SceneComponent.K2_AttachToComponent` OtherComp (`self.Sphere`) "None" "KeepWorld" "KeepWorld" "KeepWorld" true)
    (`KismetArrayLibrary.Array_Add` (`self.AttachedComponents`) OtherComp)))

(fn `CreateNewSplineMeshComponent`
  (returns (NewComponent :type "SplineMeshComponent Object Reference"))
  (bind _returnvalue (`AddComponent|NODE_AddSplineMeshComponent-0` :`bManualAttachment` true))
  (`SceneComponent.SetMobility` _returnvalue "Movable")
  (`SceneComponent.K2_AttachToComponent` _returnvalue (`self.Spline`) "None" "SnapToTarget" "SnapToTarget" "KeepWorld" false)
  (`StaticMeshComponent.SetStaticMesh` _returnvalue "/Game/Task_07/Cylinder_BB1BB71A.Cylinder_BB1BB71A")
  (`SplineMeshComponent.SetForwardAxis` _returnvalue "X" false)
  (`PrimitiveComponent.SetCollisionObjectType` _returnvalue "ECC_GameTraceChannel1")
  (`PrimitiveComponent.SetCollisionEnabled` _returnvalue "QueryAndPhysics")
  (return _returnvalue))

(fn `UpdateSplineMesh`
  (bind _spline (`self.Spline`))
  (bind _spline_2 (`self.Spline`))
  (for _index (range (`SplineComponent.GetNumberOfSplinePoints` (`self.Spline`)))
    (if (not (`KismetArrayLibrary.Array_IsValidIndex` (`self.SplineMeshes`) _index))
      (bind _newcomponent (`self.CreateNewSplineMeshComponent`))
      (`KismetArrayLibrary.Array_Add` (`self.SplineMeshes`) _newcomponent))
    (bind _returnvalue (+ _index 1))
    (`SplineMeshComponent.SetStartAndEnd` (`|GetArrayItem` (`self.SplineMeshes`) _index) (`SplineComponent.GetLocationAtSplinePoint` _spline_2 _index "Local") (`SplineComponent.GetTangentAtSplinePoint` _spline_2 _index "Local") (`SplineComponent.GetLocationAtSplinePoint` _spline _returnvalue "Local") (`SplineComponent.GetTangentAtSplinePoint` _spline _returnvalue "Local") true)))

(fn `UpdateSplinePoints`
  (for _index (range (`SplineComponent.GetNumberOfSplinePoints` (`self.Spline`)))
    (bind _returnvalue (/ (`KismetMathLibrary.Conv_IntToDouble` (+ _index 1)) (`KismetMathLibrary.Conv_IntToDouble` (`SplineComponent.GetNumberOfSplinePoints` (`self.Spline`)))))
    (bind _returnvalue_x (`KismetMathLibrary.BreakVector` (`KismetMathLibrary.VLerp` (`SceneComponent.RelativeLocation` (`self.Spline`)) (`KismetMathLibrary.InverseTransformLocation` (`self.GetTransform`) (`SceneComponent.K2_GetComponentLocation` (`self.Sphere`))) _returnvalue)))
    (bind (_returnvalue_x_2 _returnvalue_y _returnvalue_z) (`KismetMathLibrary.BreakVector` (`KismetMathLibrary.VLerp` (`SceneComponent.RelativeLocation` (`self.Spline`)) (`KismetMathLibrary.InverseTransformLocation` (`self.GetTransform`) (`SceneComponent.K2_GetComponentLocation` (`self.Sphere`))) (`KismetMathLibrary.MultiplyMultiply_FloatFloat` _returnvalue 2.0))))
    (`SplineComponent.SetLocationAtSplinePoint` (`self.Spline`) _index (`KismetMathLibrary.MakeVector` _returnvalue_x _returnvalue_y _returnvalue_z) "Local" false)))

(fn `UserConstructionScript`)