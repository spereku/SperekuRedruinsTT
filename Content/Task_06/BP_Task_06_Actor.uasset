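; BP_Task_06_Actor is a projectile actor that homes on its Origin actor.
; BeginPlay sets Origin's root component as the homing target of ProjectileMovement.
; While Origin is valid, Tick sets homing acceleration to half the distance to it, so the pull grows like a spring as the projectile strays.
; When the projectile stops, ResetProjectileMovement restarts it on the Cylinder component along the actor's forward vector at a fixed speed.
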(event `self.ReceiveBeginPlay`
  (set `ProjectileMovementComponent.HomingTargetComponent` (`Actor.RootComponent` (`self.Origin`)) (`self.ProjectileMovement`)))

(event `self.ReceiveTick`
  (params (DeltaSeconds :type "Float (single-precision)"))
  (`/Engine/EditorBlueprintResources/StandardMacros.IsValid` (`self.Origin`)
    (:`Is Valid`
      (set `ProjectileMovementComponent.HomingAccelerationMagnitude` (/ (`KismetMathLibrary.Vector_Distance` (`self.K2_GetActorLocation` (`self.Origin`)) (`self.K2_GetActorLocation`)) 2.0) (`self.ProjectileMovement`)))))

(event `self.ProjectileMovement.OnProjectileStop`
  (params (ImpactResult :type "HitResult Structure (by ref)"))
  (`CPP_GenericFL.ResetProjectileMovement` (`self.ProjectileMovement`) (`self.Cylinder`) (* (`self.GetActorForwardVector`) 1500.0)))

(fn `UserConstructionScript`)