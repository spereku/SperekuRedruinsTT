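; Player character that rides along a Trajectory spline and launches physics balls with an aim preview.
; Each tick it loops along the spline at a normalized speed adjustable with the Add and Subtract keys.
; Holding left mouse predicts the projectile path, drawing debug spheres and moving a spawned BP_HitPlace marker to the predicted impact.
; Releasing spawns a BP_PhysicBall launched along the control rotation.
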(event `self.ReceiveBeginPlay`
  (bind _returnvalue (`|SpawnActorFromClass` "/Game/Task_05/BP_HitPlace.BP_HitPlace_C" (`KismetMathLibrary.MakeTransform` (0.0 0.0 0.0)) "Undefined" "MultiplyWithRoot" null null))
  (bind _output_get (set `self.HitPlane` _returnvalue))
  (`self.SetActorHiddenInGame` _output_get true)
  (`self.SetActorEnableCollision` (`self.HitPlane`) false))

(event `self.ReceiveTick`
  (params (DeltaSeconds :type "Float (single-precision)"))
  (`self.MoveAlongSpline` DeltaSeconds)
  (`self.DrawPredictionPath`))

(event `Key|Add`
  (params (Key :type "Key Structure"))
  (:`Pressed`
    (set `self.DefaultMoveSpeed` (`KismetMathLibrary.FClamp` (+ (`self.DefaultMoveSpeed`) (`self.MoveSpeedStep`))))))

(event `Key|Subtract`
  (params (Key :type "Key Structure"))
  (:`Pressed`
    (set `self.DefaultMoveSpeed` (`KismetMathLibrary.FClamp` (- (`self.DefaultMoveSpeed`) (`self.MoveSpeedStep`)) 0.0 1.0))))

(event `Key|LeftMouseButton`
  (params (Key :type "Key Structure"))
  (:`Pressed`
    (set `self.LeftMouseButtonPressed` true))
  (:`Released`
    (set `self.LeftMouseButtonPressed` false)
    (bind _returnvalue (`|SpawnActorFromClass` "/Game/Task_05/BP_PhysicBall.BP_PhysicBall_C" (`KismetMathLibrary.MakeTransform` (`SceneComponent.K2_GetComponentLocation` (`self.ProjectileSpawnLocation`)) (`self.GetControlRotation`) (0.3 0.3 0.3)) "AlwaysSpawn" "MultiplyWithRoot" null null))
    (`ProjectileMovementComponent.SetVelocityInLocalSpace` (`/Game/Task_05/BP_PhysicBall.ProjectileMovement` _returnvalue) (`KismetMathLibrary.MakeVector` (`self.ProjectileVelocity`)))))

(fn `DrawPredictionPath`
  (if (`self.LeftMouseButtonPressed`)
    (bind (_outhit _outpathpositions _outlasttracedestination _returnvalue) (`GameplayStatics.Blueprint_PredictProjectilePath_ByObjectType` (`SceneComponent.K2_GetComponentLocation` (`self.ProjectileSpawnLocation`)) (* (`KismetMathLibrary.GetForwardVector` (`self.GetControlRotation`)) (`self.ProjectileVelocity`)) true 30.0 (`|MakeArray` "ObjectTypeQuery1" "ObjectTypeQuery2" :!type "EObjectTypeQuery Enum") false (`|MakeArray` self :!type "Actor Object Reference")))
    (for _array_element _outpathpositions
      (`KismetSystemLibrary.DrawDebugSphere` _array_element 20.0 12 (struct :`R` 1.0 :`A` 1.0) 0.0 1.0))
    (if _returnvalue
      (`self.SetActorHiddenInGame` (`self.HitPlane`) false)
      (`self.K2_SetActorLocation` (`self.HitPlane`) (- (`.Location` (`GameplayStatics.BreakHitResult` _outhit)) (0.0 0.0 30.0)) false false)
      (else
        (`self.SetActorHiddenInGame` (`self.HitPlane`) true)))))

(fn `MoveAlongSpline`
  (params (DeltaSeconds :type "Float (double-precision)"))
  (`self.Trajectory`
    (:`then`
      (set `self.MoveTime` (mod (+ (`self.MoveTime`) (* DeltaSeconds (`self.DefaultMoveSpeed`))) 1.0))
      (`self.K2_SetActorLocation` (+ (`SplineComponent.GetLocationAtTime` (`/Game/Task_05/BP_Trajectory.Spline` (`self.Trajectory`)) (`self.MoveTime`) "World" false) (0.0 0.0 100.0))))
    (:`else`)))

(fn `UserConstructionScript`)